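; Installment_bool_02_BP is a one-time build spot where a construction rubble mesh is replaced by a built cube.
; The cube starts hidden, and TraceHit and SetHidden toggle the rubble between a hologram material and its original, cached in the construction script.
; ActionBuild runs once, setting Lock to stop highlight changes, then applies the ChangeTo material to the cube, reveals it and destroys the rubble component.
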(event `self.ReceiveBeginPlay`
  (`SceneComponent.SetHiddenInGame` (`self.Cube`) true false))

(event `/Game/Machanics_BPs/Interact_BPI.Trace_hit`
  (if (not (`self.Lock`))
    (`PrimitiveComponent.SetMaterial` (`self.Construction_Rubble_LOD0_risqG`) 0 "/Game/Machanics_BPs/installment/1/hologram.hologram")))

(event `/Game/Machanics_BPs/Interact_BPI.Set_hidden`
  (if (not (`self.Lock`))
    (`PrimitiveComponent.SetMaterial` (`self.Construction_Rubble_LOD0_risqG`) 0 (`self.original_material`))))

(event `/Game/Machanics_BPs/Interact_BPI.Action_build`
  (`/Engine/EditorBlueprintResources/StandardMacros.DoOnce` false
    (:`Completed`
      (set `self.Lock` true)
      (`PrimitiveComponent.SetMaterial` (`self.Cube`) 0 (`self.change_to`))
      (`SceneComponent.SetHiddenInGame` (`self.Cube`) false false)
      (`ActorComponent.K2_DestroyComponent` (`self.Construction_Rubble_LOD0_risqG`)))))

(fn `UserConstructionScript`
  (set `self.original_material` (`PrimitiveComponent.GetMaterial` (`self.Construction_Rubble_LOD0_risqG`) 0)))