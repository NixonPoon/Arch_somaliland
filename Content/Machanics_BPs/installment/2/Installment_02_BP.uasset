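; Installment_02_BP is a buildable repair spot that turns broken wall and cinder block rubble into a finished piece.
; TraceHit reveals the Cube as a preview, and SetHidden or force_hidden hides it, until the Lock flag is set.
; ActionBuild runs once, setting Lock, applying the final material to the Cube and destroying the three broken meshes.
; An unconnected delayed check against the first-person character's SelectedPart never runs.
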(event `/Game/Machanics_BPs/Interact_BPI.Trace_hit`
  (if (not (`self.lock`))
    (`SceneComponent.SetHiddenInGame` (`self.Cube`) false false)))

(event `/Game/Machanics_BPs/Interact_BPI.Set_hidden`
  (if (not (`self.lock`)) :!label _label
    (`SceneComponent.SetHiddenInGame` (`self.Cube`) true false)))

(event `force_hidden`
  (goto _label))

(event `/Game/Machanics_BPs/Interact_BPI.Action_build`
  (`/Engine/EditorBlueprintResources/StandardMacros.DoOnce` false
    (:`Completed`
      (set `self.lock` true)
      (`PrimitiveComponent.SetMaterial` (`self.Cube`) 0 "/Game/Megascans/Surfaces/Damaged_Brick_Wall_vmdkahflw/Albedo_4K_vmdkahflw_Mat.Albedo_4K_vmdkahflw_Mat")
      (`ActorComponent.K2_DestroyComponent` (`self.Broken_Wall_LOD0_slunl`))
      (`ActorComponent.K2_DestroyComponent` (`self.Broken_Wall_LOD0_slvfI`))
      (`ActorComponent.K2_DestroyComponent` (`self.Broken_Cinder_Blocks_LOD0_rieq0_3`)))))

(fn `UserConstructionScript`)