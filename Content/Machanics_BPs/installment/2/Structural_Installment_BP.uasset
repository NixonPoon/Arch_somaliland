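; Placeable structural installment that previews as a hologram and becomes a permanent structure when built.
; The construction script applies the hologram material, and the mesh stays hidden until TraceHit receives this actor as the selection, with SetHidden hiding it again.
; ActionBuild runs once, locking the piece against hiding, swapping to the build material and destroying the actors in WorldObject.
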(event `self.ReceiveBeginPlay`
  (`SceneComponent.SetHiddenInGame` (`self.Mesh`) true false))

(event `/Game/Machanics_BPs/Interact_BPI.Trace_hit`
  (params (selected_actor :type "Actor Object Reference"))
  (if (`self.lock`)
    (`SceneComponent.SetHiddenInGame` (`self.Mesh`) false false :!label _label)
    (elif (== selected_actor self)
      (goto _label))))

(event `/Game/Machanics_BPs/Interact_BPI.Set_hidden`
  (if (not (`self.lock`))
    (`SceneComponent.SetHiddenInGame` (`self.Mesh`) true false)))

(event `/Game/Machanics_BPs/Interact_BPI.Action_build`
  (`/Engine/EditorBlueprintResources/StandardMacros.DoOnce` false
    (:`Completed`
      (set `self.lock` true)
      (`PrimitiveComponent.SetMaterial` (`self.Mesh`) 0 (`self.build_material`))
      (for _array_element (`self.World_object`)
        (`self.K2_DestroyActor` _array_element)))))

(fn `UserConstructionScript`
  (`PrimitiveComponent.SetMaterial` (`self.Mesh`) 0 "/Game/Machanics_BPs/installment/1/hologram.hologram"))