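; Clearable actor that previews as a hologram when selected and removes itself when the build action runs.
; It caches mesh materials on BeginPlay; TraceHit applies Hologram to slot 0 if it is selected or Lock is set.
; SetHidden reapplies cached materials unless locked, writing each to slot 0 so the last one remains.
; ActionBuild runs once, hiding the actor and destroying it a second later.
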(event `self.ReceiveBeginPlay`
  (set `self.local_material` (`MeshComponent.GetMaterials` (`self.Mesh`))))

(event `/Game/Machanics_BPs/Interact_BPI.Trace_hit`
  (params (selected_actor :type "Actor Object Reference"))
  (if (`self.lock`)
    (`PrimitiveComponent.SetMaterial` (`self.Mesh`) 0 "/Game/Machanics_BPs/installment/1/hologram.hologram" :!label _label)
    (elif (== selected_actor self)
      (goto _label))))

(event `/Game/Machanics_BPs/Interact_BPI.Set_hidden`
  (if (not (`self.lock`))
    (for _array_element (`self.local_material`)
      (`PrimitiveComponent.SetMaterial` (`self.Mesh`) 0 _array_element))))

(event `/Game/Machanics_BPs/Interact_BPI.Action_build`
  (`/Engine/EditorBlueprintResources/StandardMacros.DoOnce` false
    (:`Completed`
      (`self.SetActorHiddenInGame` true)
      (`KismetSystemLibrary.Delay` 1.0)
      (`self.K2_DestroyActor`))))

(fn `UserConstructionScript`)