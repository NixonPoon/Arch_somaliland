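; Rubble actor for an installment mechanic that highlights when traced and is removed by a build action.
; The construction script caches the rubble mesh's first material.
; TraceHit swaps that slot to a Hologram material, and SetHidden restores the cached original.
; ActionBuild simply destroys the actor.
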(event `/Game/Machanics_BPs/Interact_BPI.Trace_hit`
  (`PrimitiveComponent.SetMaterial` (`self.Construction_Rubble_LOD0_risqG`) 0 "/Game/Machanics_BPs/installment/1/hologram.hologram"))

(event `/Game/Machanics_BPs/Interact_BPI.Set_hidden`
  (`PrimitiveComponent.SetMaterial` (`self.Construction_Rubble_LOD0_risqG`) 0 (`self.original_material`)))

(event `/Game/Machanics_BPs/Interact_BPI.Action_build`
  (`self.K2_DestroyActor`))

(fn `UserConstructionScript`
  (set `self.original_material` (`PrimitiveComponent.GetMaterial` (`self.Construction_Rubble_LOD0_risqG`) 0)))