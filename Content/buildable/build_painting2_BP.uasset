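; Buildable painting Blueprint for the first-person building system, with a mesh component named SMChair.
; AskforAvaliableMode copies its floor, wall and ceiling snap flags onto the player's FirstPersonCharacter.
; BeginPlay loops over the mesh's materials, keeping only the last one.
; CustomizeHit puts a delete-highlight material on slot 0, and SetHidden sets that slot to the stored material.
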(event `/Game/Machanics_BPs/Interact_BPI.Ask_for_avaliable_mode`
  (bind _asfirst_person_character (cast `/Game/FirstPersonBP/Blueprints/FirstPersonCharacter` (`GameplayStatics.GetPlayerCharacter` 0)))
  (set `/Game/FirstPersonBP/Blueprints/FirstPersonCharacter.Can_SnapFloor` (`self.Snap to ground`) _asfirst_person_character)
  (set `/Game/FirstPersonBP/Blueprints/FirstPersonCharacter.Can_SnapWall` (`self.Snap to wall`) _asfirst_person_character)
  (set `/Game/FirstPersonBP/Blueprints/FirstPersonCharacter.Can_SnapCeil` (`self.Snap to ceil`) _asfirst_person_character))

(event `self.ReceiveBeginPlay`
  (for _array_element (`MeshComponent.GetMaterials` (`self.SM_Chair`))
    (set `self.Material` _array_element)))

(event `/Game/Machanics_BPs/Interact_BPI.Customize_hit`
  (`PrimitiveComponent.SetMaterial` (`self.SM_Chair`) 0 "/Game/buildable/m_build_highlight_delete.m_build_highlight_delete"))

(event `/Game/Machanics_BPs/Interact_BPI.Set_hidden`
  (`PrimitiveComponent.SetMaterial` (`self.SM_Chair`) 0 (`self.Material`)))

(fn `UserConstructionScript`)